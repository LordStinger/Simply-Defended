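; Factory tower that earns the player money about once per second, using a Delay on Tick, and can be upgraded for a cost.
; Upgrade checks level and funds, raises the level and deducts the cost from the NewPlayerController found at BeginPlay.
; AdjustToLevel sets doubling income and rising cost through level 5, refreshing level and MPS text.
; Level 6 is reachable but keeps the previous income and labels.
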(event Custom|UpgradeTower
  (Variables|Default|SetTowerLevel (+ (Variables|Default|GetTowerLevel) 1))
  (CallFunction|AdjusttoLevel))

(event Custom|AdjustToLevel
  (bind _towerlevel (Variables|Default|GetTowerLevel))
  (if (== _towerlevel 1)
    (Variables|Default|SetMoneyToAdd 2)
    (Variables|Default|SetCostToUpgrade 100)
    (CallFunction|UpdateLevelText :!label _label)
    (elif (== _towerlevel 2)
      (Variables|Default|SetMoneyToAdd 4)
      (Variables|Default|SetCostToUpgrade 200)
      (goto _label)
      (elif (== _towerlevel 3)
        (Variables|Default|SetMoneyToAdd 8)
        (Variables|Default|SetCostToUpgrade 300)
        (goto _label)
        (elif (== _towerlevel 4)
          (Variables|Default|SetMoneyToAdd 16)
          (Variables|Default|SetCostToUpgrade 400)
          (goto _label)
          (elif (== _towerlevel 5)
            (Variables|Default|SetMoneyToAdd 32)
            (Variables|Default|SetCostToUpgrade 500)
            (goto _label)
            (elif (not (== _towerlevel 6))
              (Variables|Default|SetMoneyToAdd 64))))))))

(event Custom|Upgrade
  (bind _playerref (Variables|Default|GetPlayerRef))
  (if (<= (Variables|Default|GetTowerLevel) 5)
    (if (<= (Variables|Default|GetCostToUpgrade) (Variables|/Game/PlayerController/NewPlayerController.NewPlayerController_C|GetMoney _playerref))
      (CallFunction|UpgradeTower)
      (Variables|/Game/PlayerController/NewPlayerController.NewPlayerController_C|SetMoney _playerref (- (Variables|/Game/PlayerController/NewPlayerController.NewPlayerController_C|GetMoney _playerref) (Variables|Default|GetCostToUpgrade)))
      (else
        (Development|PrintString "You Do Not Have Enough Money!")))
    (else
      (Development|PrintString "Already Max Level!"))))

(event Custom|UpdateLevelText
  (bind _output_get (Variables|Default|SetLevelTextsd "Level: "))
  (Rendering|Components|TextRender|SetText (Variables|Default|GetLevelText) (Utilities|Text|ToText(String) (Utilities|String|Append _output_get (Utilities|String|ToString(Integer) (Variables|Default|GetTowerLevel)))))
  (bind _output_get_2 (Variables|Default|SetLevelTextsd "MPS: "))
  (Rendering|Components|TextRender|SetText (Variables|Default|GetMPS) (Utilities|Text|ToText(String) (Utilities|String|Append _output_get_2 (Utilities|String|ToString(Integer) (Variables|Default|GetMoneyToAdd))))))

(event EventTick
  (params (DeltaSeconds :type Float%20%28single-precision%29))
  (bind _playerref (Variables|Default|GetPlayerRef))
  (Utilities|FlowControl|Delay 1.0)
  (Variables|/Game/PlayerController/NewPlayerController.NewPlayerController_C|SetMoney _playerref (+ (Variables|/Game/PlayerController/NewPlayerController.NewPlayerController_C|GetMoney _playerref) (Variables|Default|GetMoneyToAdd))))

(event EventBeginPlay
  (bind _outactors (Actor|GetAllActorsOfClass "/Game/PlayerController/NewPlayerController.NewPlayerController_C"))
  (Variables|Default|SetPlayerRef (Utilities|Array|Get(acopy) _outactors))
  (CallFunction|AdjusttoLevel))

(fn ConstructionScript)
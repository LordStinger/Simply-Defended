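; Gunner tower Blueprint that automatically fires projectiles at the nearest enemy within its attack range.
; While Firerate is at most one, Tick searches all EnemyCharacter actors for the closest and checks its distance.
; A Delay on Tick spaces the shots, then a GunnerProjectile spawns at FirePoint with the target passed in.
; The projectile's target reference is cleared immediately after spawning.
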(event EventTick
  (params (DeltaSeconds :type Float%20%28single-precision%29))
  (bind _firepoint (Variables|Default|GetFirePoint))
  (if (<= (Variables|Default|GetFirerate) 1.0)
    (bind _outactors (Actor|GetAllActorsOfClass "/Game/Enemies/EnemyCharacter.EnemyCharacter_C"))
    (bind _output_get (Variables|Default|SetTargetEnemy (.ReturnValue (Actor|FindNearestActor (Transformation|GetWorldLocation (Variables|Default|GetDefaultSceneRoot)) _outactors))))
    (if (<= (.Distance (Actor|FindNearestActor (Transformation|GetWorldLocation (Variables|Default|GetDefaultSceneRoot)) _outactors)) (Variables|Default|GetAttackRange))
      (Utilities|FlowControl|Delay 0.5)
      (bind _returnvalue (Game|SpawnActorfromClass "/Game/Towers/GunnerProjectile.GunnerProjectile_C" (Math|Transform|MakeTransform (Transformation|GetWorldLocation _firepoint) (Transformation|GetWorldRotation _firepoint)) "Undefined" "MultiplyWithRoot" 0 _output_get 0))
      (bind _output_get_2 (Variables|Default|SetProjectileRef _returnvalue))
      (Variables|/Game/Towers/GunnerProjectile.GunnerProjectile_C|SetTargetEnemyRef _output_get_2 0))))

(fn ConstructionScript)
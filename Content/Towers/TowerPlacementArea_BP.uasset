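; Tower build zone actor where the player buys and upgrades one Gunner, Sniper or Factory tower.
; Box overlap toggles the highlight and registers the zone with NewPlayerController, the player pawn.
; Purchase events mark the zone occupied before checking money, then deduct the cost and spawn the tower at PlacementPoint.
; Upgrade events forward to the stored tower, and SetCurrentTowerStats caches its stats and upgrade cost on the zone.
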(event OnComponentBeginOverlap(Box)
  (params (OverlappedComponent :type Primitive%20Component%20Object%20Reference) (OtherActor :type Actor%20Object%20Reference) (OtherComp :type Primitive%20Component%20Object%20Reference) (OtherBodyIndex :type Integer) (bFromSweep :type Boolean) (SweepResult :type Hit%20Result%20Structure%20%28by%20ref%29))
  (if (Components|ComponentHasTag OtherComp "Player")
    (Rendering|SetVisibility (Variables|Default|GetAreaHighlighter) true false)
    (bind _asnew_player_controller (Utilities|Casting|CastToNewPlayerController (Game|Player|GetPlayerPawn 0))
      (:then
        (Variables|Default|SetCharacterIsOverlapping true)
        (Development|PrintString "Player has entered a Build Zone.")
        (CallFunction|RunCast)
        (CallFunction|SetCurrentTowerStats))
      (:CastFailed
        (Development|PrintString "Cast to player FAILED!")
        (Variables|/Game/PlayerController/NewPlayerController.NewPlayerController_C|SetInBuildZone _asnew_player_controller true)))))

(event OnComponentEndOverlap(Box)
  (params (OverlappedComponent :type Primitive%20Component%20Object%20Reference) (OtherActor :type Actor%20Object%20Reference) (OtherComp :type Primitive%20Component%20Object%20Reference) (OtherBodyIndex :type Integer))
  (if (Components|ComponentHasTag OtherComp "Player")
    (Rendering|SetVisibility (Variables|Default|GetAreaHighlighter) false false)
    (Variables|Default|SetCharacterIsOverlapping false)
    (bind _asnew_player_controller (Utilities|Casting|CastToNewPlayerController (Game|Player|GetPlayerPawn 0))
      (:then
        (Development|PrintString "Player has left a Build Zone.")
        (Variables|/Game/PlayerController/NewPlayerController.NewPlayerController_C|SetInBuildZone _asnew_player_controller false)
        (CallFunction|RunCast)
        (Variables|Default|SetTowerCurrentLevel 0.0)
        (Variables|Default|SetTowerCurrentDamage 0.0)
        (Variables|Default|SetTowerCurrentFirerate 0.0)
        (Variables|Default|SetTowerCurrentRange 0.0)
        (Variables|Default|SetFactoryCurrentLevel 0.0)
        (Variables|Default|SetFactoryCurrentMPS 0.0)
        (Variables|Default|SetCostToUpgrade 0)
        (Default|ResetNextStats (Variables|Default|GetPlayerRef)))
      (:CastFailed
        (Development|PrintString "Cast to player FAILED!")
        (Variables|/Game/PlayerController/NewPlayerController.NewPlayerController_C|SetInBuildZone (stale OnComponentBeginOverlap(Box) _asnew_player_controller) true)))))

(event Custom|RunCast
  (bind _returnvalue (Game|Player|GetPlayerPawn 0))
  (if (Variables|Default|GetCharacterIsOverlapping)
    (bind _asnew_player_controller (Utilities|Casting|CastToNewPlayerController _returnvalue))
    (Variables|/Game/PlayerController/NewPlayerController.NewPlayerController_C|SetCurrentPlacementArea _asnew_player_controller self)
    (bind _output_get (Variables|Default|SetAs%20New%20Player%20Controller _asnew_player_controller))
    (Variables|/Game/PlayerController/NewPlayerController.NewPlayerController_C|SetInBuildZone _output_get true)
    (Default|UpdateBuildText _output_get)
    (Development|PrintString "IN BUILD ZONE")
    (else
      (bind _asnew_player_controller_2 (Utilities|Casting|CastToNewPlayerController _returnvalue))
      (bind _output_get_2 (Variables|Default|SetAs%20New%20Player%20Controller _asnew_player_controller_2))
      (Variables|/Game/PlayerController/NewPlayerController.NewPlayerController_C|SetInBuildZone _output_get_2 false)
      (Default|UpdateBuildText _output_get_2)
      (Development|PrintString "NOT IN BULD ZONE"))))

(event Custom|SetGunnerAsActiveTower
  (if (Variables|Default|GetIsOccupied)
    (Development|PrintString "A Tower Is Already Place Here!")
    (else
      (Variables|Default|SetIsOccupied true)
      (if (>= (Variables|/Game/PlayerController/NewPlayerController.NewPlayerController_C|GetMoney (Variables|Default|GetPlayerRef)) 1e+03)
        (Variables|/Game/PlayerController/NewPlayerController.NewPlayerController_C|SetMoney (Variables|Default|GetPlayerRef) (- (Variables|/Game/PlayerController/NewPlayerController.NewPlayerController_C|GetMoney (Variables|Default|GetPlayerRef)) 1e+03))
        (bind _returnvalue (Game|SpawnActorfromClass "/Game/Towers/GunnerTower_BP.GunnerTower_BP_C" (Math|Transform|MakeTransform (Transformation|GetWorldLocation (Variables|Default|GetPlacementPoint)) (Transformation|GetWorldRotation (Variables|Default|GetPlacementPoint))) "Undefined" "MultiplyWithRoot" 0 1e+01 0))
        (Variables|Default|SetGunnerTowerRef _returnvalue)
        (Variables|Default|SetGunnerTowerBool true)
        (CallFunction|SetCurrentTowerStats)
        (else
          (Development|PrintString "Not Enough Money"))))))

(event Custom|SetSniperAsActiveTower
  (if (Variables|Default|GetIsOccupied)
    (Development|PrintString "A Tower Is Already Place Here!")
    (else
      (Variables|Default|SetIsOccupied true)
      (if (>= (Variables|/Game/PlayerController/NewPlayerController.NewPlayerController_C|GetMoney (Variables|Default|GetPlayerRef)) 1e+03)
        (Variables|/Game/PlayerController/NewPlayerController.NewPlayerController_C|SetMoney (Variables|Default|GetPlayerRef) (- (Variables|/Game/PlayerController/NewPlayerController.NewPlayerController_C|GetMoney (Variables|Default|GetPlayerRef)) 1e+03))
        (bind _returnvalue (Game|SpawnActorfromClass "/Game/Towers/SniperTower_BP.SniperTower_BP_C" (Math|Transform|MakeTransform (Transformation|GetWorldLocation (Variables|Default|GetPlacementPoint)) (Transformation|GetWorldRotation (Variables|Default|GetPlacementPoint))) "Undefined" "MultiplyWithRoot" 0 1e+02 0))
        (Variables|Default|SetSniperTowerRef _returnvalue)
        (Variables|Default|SetSniperTowerBool true)
        (CallFunction|SetCurrentTowerStats)
        (else
          (Development|PrintString "Not Enough Money"))))))

(event Custom|SetFactoryAsActiveTower
  (if (Variables|Default|GetIsOccupied)
    (Development|PrintString "A Tower Is Already Place Here!")
    (else
      (Variables|Default|SetIsOccupied true)
      (if (>= (Variables|/Game/PlayerController/NewPlayerController.NewPlayerController_C|GetMoney (Variables|Default|GetPlayerRef)) 1.5e+03)
        (Variables|/Game/PlayerController/NewPlayerController.NewPlayerController_C|SetMoney (Variables|Default|GetPlayerRef) (- (Variables|/Game/PlayerController/NewPlayerController.NewPlayerController_C|GetMoney (Variables|Default|GetPlayerRef)) 1.5e+03))
        (bind _returnvalue (Game|SpawnActorfromClass "/Game/Towers/FactoryTower_BP.FactoryTower_BP_C" (Math|Transform|MakeTransform (Transformation|GetWorldLocation (Variables|Default|GetPlacementPoint)) (Transformation|GetWorldRotation (Variables|Default|GetPlacementPoint))) "Undefined" "MultiplyWithRoot" 0 0))
        (Variables|Default|SetFactoryTowerRef _returnvalue)
        (Variables|Default|SetFactoryTowerBool true)
        (CallFunction|SetCurrentTowerStats)
        (else
          (Development|PrintString "Not Enough Money"))))))

(event Custom|ClearActiveTower
  (Variables|Default|SetIsOccupied false))

(event Custom|UpgradeGunnerTower
  (Default|GunnerUpgrade (Variables|Default|GetGunnerTowerRef))
  (CallFunction|SetCurrentTowerStats))

(event Custom|UpgradeFactoryTower
  (Default|Upgrade (Variables|Default|GetFactoryTowerRef))
  (CallFunction|SetCurrentTowerStats))

(event Custom|UpgradeSniperTower
  (Default|SniperUpgrade (Variables|Default|GetSniperTowerRef))
  (CallFunction|SetCurrentTowerStats))

(event Custom|SetCurrentTowerStats
  (bind _gunnertowerref (Variables|Default|GetGunnerTowerRef))
  (bind _factorytowerref (Variables|Default|GetFactoryTowerRef))
  (bind _snipertowerref (Variables|Default|GetSniperTowerRef))
  (if (Variables|Default|GetSniperTowerBool)
    (Variables|Default|SetTowerCurrentLevel (Math|Conversions|ToFloat(Integer) (Variables|/Game/Towers/SniperTower_BP.SniperTower_BP_C|GetTowerLevel _snipertowerref)))
    (Variables|Default|SetTowerCurrentDamage (Variables|/Game/Towers/SniperTower_BP.SniperTower_BP_C|GetDamage _snipertowerref))
    (Variables|Default|SetTowerCurrentFirerate (Variables|/Game/Towers/SniperTower_BP.SniperTower_BP_C|GetFirerate _snipertowerref))
    (Variables|Default|SetTowerCurrentRange (Variables|/Game/Towers/SniperTower_BP.SniperTower_BP_C|GetAttackRange _snipertowerref))
    (Variables|Default|SetCostToUpgrade (Variables|/Game/Towers/SniperTower_BP.SniperTower_BP_C|GetCostToUpgrade _snipertowerref))
    (elif (Variables|Default|GetFactoryTowerBool)
      (Variables|Default|SetFactoryCurrentLevel (Math|Conversions|ToFloat(Integer) (Variables|/Game/Towers/FactoryTower_BP.FactoryTower_BP_C|GetTowerLevel _factorytowerref)))
      (Variables|Default|SetFactoryCurrentMPS (Math|Conversions|ToFloat(Integer) (Variables|/Game/Towers/FactoryTower_BP.FactoryTower_BP_C|GetMoneyToAdd _factorytowerref)))
      (Variables|Default|SetCostToUpgrade (Variables|/Game/Towers/FactoryTower_BP.FactoryTower_BP_C|GetCostToUpgrade _factorytowerref))
      (elif (Variables|Default|GetGunnerTowerBool)
        (Variables|Default|SetTowerCurrentLevel (Math|Conversions|ToFloat(Integer) (Variables|/Game/Towers/GunnerTower_BP.GunnerTower_BP_C|GetTowerLevel _gunnertowerref)))
        (Variables|Default|SetTowerCurrentDamage (Variables|/Game/Towers/GunnerTower_BP.GunnerTower_BP_C|GetDamage _gunnertowerref))
        (Variables|Default|SetTowerCurrentFirerate (Variables|/Game/Towers/GunnerTower_BP.GunnerTower_BP_C|GetFirerate _gunnertowerref))
        (Variables|Default|SetTowerCurrentRange (Variables|/Game/Towers/GunnerTower_BP.GunnerTower_BP_C|GetAttackRange _gunnertowerref))
        (Variables|Default|SetCostToUpgrade (Variables|/Game/Towers/GunnerTower_BP.GunnerTower_BP_C|GetCostToUpgrade _gunnertowerref))))))

(event EventBeginPlay
  (Rendering|SetVisibility (Variables|Default|GetAreaHighlighter) false false)
  (bind _outactors (Actor|GetAllActorsOfClass "/Game/PlayerController/NewPlayerController.NewPlayerController_C"))
  (Variables|Default|SetPlayerRef (Utilities|Array|Get(acopy) _outactors))
  (bind _foundwidgets (Widget|GetAllWidgetsOfClass "/Game/UI/BuyMenuWidget.BuyMenuWidget_C" false))
  (Variables|Default|SetBuyMenuRef (Utilities|Array|Get(acopy) _foundwidgets)))

(fn ConstructionScript)